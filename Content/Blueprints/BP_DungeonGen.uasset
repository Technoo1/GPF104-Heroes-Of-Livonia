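; Procedural dungeon generator that builds a tile-based room layout in the Construction Script from a seeded random stream, with a NewSeed toggle to reroll.
; GenerateMap chains rooms by stepping from the previous one in a random choice of eight directions, testing for occupied tiles.
; Each room is a random-sized grid with optional random floor culling, though that loop's connectivity and exit logic looks unfinished.
; SpawnTiles places the collected tiles as scaled-position mesh instances.
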(event Custom|Generate%20Map
  (for _index (range 0 (- (Variables|MapSettings|GetRoomCount) 1))
    (if (== _index 0)
      (bind (_floortiles _location_ _extents) (CallFunction|RoomMakeFloorArea (Variables|Default|GetPrevLocation)))
      (Variables|Default|SetFloorTiles _floortiles)
      (Utilities|Map|Add (Variables|Default|GetRooms) _location_ _extents)
      (else
        (bind (_valid_ _newlocation_) (CallFunction|RoomFindNextLocation))
        (if _valid_
          (bind _output_get (Variables|Default|SetNextLocation _newlocation_))
          (bind (_floortiles_2 _location__2 _extents_2) (CallFunction|RoomMakeFloorArea _output_get))
          (Utilities|Array|AppendArray (Variables|Default|GetFloorTiles) _floortiles_2)
          (Utilities|Map|Add (Variables|Default|GetRooms) _location__2 _extents_2)
          (Variables|Default|SetPrevLocation (Variables|Default|GetNextLocation))))))
  (CallFunction|SpawnTiles))

(fn ConstructionScript
  (Utilities|FlowControl|Sequence
    (:then_0
      ;[1 1 1] On Click "NewSeed" get new random seed
      (if (Variables|EditorTools|GetNewSeed)
        (Variables|EditorTools|SetNewSeed false)
        (bind _output_get (Variables|MapSettings|SetSeed (Math|Random|RandomInteger 900000)))
        (Math|Random|SetRandomStreamSeed (Variables|EditorTools|GetStream) _output_get)))
    (:then_1
      ;[1 1 1] Manually update stream with seed
      (Math|Random|SetRandomStreamSeed (Variables|EditorTools|GetStream) (Variables|MapSettings|GetSeed)))
    (:then_2
      (CallFunction|GenerateMap))))

(fn RoomMakeFloorArea
  (params (Location :type Int%20Vector%20Structure))
  (bind _roomsize_min (Variables|MapSettings|GetRoomSize_Min))
  (bind _roomsize_max (Variables|MapSettings|GetRoomSize_Max))
  (bind _stream (Variables|EditorTools|GetStream))
  ;[1 1 1] Get Random X annd Y extents and make array of floor tiles from X, Y added to root position
  (LocalVariables|SetRootLocation Location)
  (LocalVariables|SetOut_X (Math|Random|RandomIntegerinRangefromStream _stream _roomsize_min _roomsize_max))
  (LocalVariables|SetOut_Y (Math|Random|RandomIntegerinRangefromStream _stream _roomsize_min _roomsize_max))
  (for _index (range 0 (- (* (LocalVariables|GetOut_X) (LocalVariables|GetOut_Y)) 1))
    (Utilities|Array|Add (LocalVariables|GetTiles) (Utilities|Struct|MakeIntVector (+ (/ _index (LocalVariables|GetOut_Y)) (.X (Utilities|Struct|BreakIntVector (LocalVariables|GetRootLocation)))) (+ (Math|Integer|%(Integer) _index (LocalVariables|GetOut_Y)) (.Y (Utilities|Struct|BreakIntVector (LocalVariables|GetRootLocation)))) (.Z (Utilities|Struct|BreakIntVector (LocalVariables|GetRootLocation))))))
  (if (Variables|MapSettings|GetFloorCulling?)
    (while (LocalVariables|GetWorking)
      ;[1 1 1] Randomly Remove Tiles from floor
      (LocalVariables|SetTiles%20Copy (LocalVariables|GetTiles))
      (for _index_2 (range 0 (Math|Integer|Clamp(Integer) (- (Math|Random|RandomIntegerinRangefromStream (Variables|EditorTools|GetStream) (Variables|MapSettings|GetFloorCull_Min) (Variables|MapSettings|GetFloorCull_Max)) 1) 0 (/ (Utilities|Array|Length (LocalVariables|GetTiles%20Copy)) 4)))
        (Utilities|Array|RemoveIndex (LocalVariables|GetTiles%20Copy) (Class|KismetMathLibrary|RandomIntegerfromStream (Variables|EditorTools|GetStream) (Utilities|Array|LastIndex (LocalVariables|GetTiles%20Copy)))))
      (Utilities|Array|Clear (LocalVariables|GetConnectedTiles))
      (Utilities|Array|Add (LocalVariables|GetConnectedTiles) (Utilities|Array|Get(acopy) (LocalVariables|GetTiles%20Copy)))
      (while false
        _))
    ;[1 1 1] Get Outer extents of room and output final results
    (for _array_element (LocalVariables|GetConnectedTiles)
      (Utilities|Array|Add (LocalVariables|GetExtent_X) (.X (Utilities|Struct|BreakIntVector _array_element)))
      (Utilities|Array|Add (LocalVariables|GetExtent_Y) (.Y (Utilities|Struct|BreakIntVector _array_element))))
    (return (LocalVariables|GetConnectedTiles) (LocalVariables|GetRootLocation) (Utilities|Struct|MakeIntVector (.MaxValue (Math|Integer|MaxOfIntArray (LocalVariables|GetExtent_X))) (.IndexOfMaxValue (Math|Integer|MaxOfIntArray (LocalVariables|GetExtent_Y)))))
    (else
      (LocalVariables|SetConnectedTiles (LocalVariables|GetTiles)))))

(fn SpawnTiles
  (for _array_element (Variables|Default|GetFloorTiles)
    (Components|InstancedStaticMesh|AddInstance (Variables|Default|GetFloor) (Math|Transform|MakeTransform (* (Math|Conversions|ToVector(Float) _array_element) (Variables|EditorTools|GetScale)) "0, 0, 0" "1.000000,1.000000,1.000000") false)))

(fn RoomFindNextLocation
  (bind _prevlocation (Variables|Default|GetPrevLocation))
  (bind _roomsize_max (Variables|MapSettings|GetRoomSize_Max))
  (bind _merging (Variables|MapSettings|GetMerging))
  (bind _prevlocation_2 (Variables|Default|GetPrevLocation))
  (bind _prevlocation_3 (Variables|Default|GetPrevLocation))
  (bind _prevlocation_4 (Variables|Default|GetPrevLocation))
  (bind _prevlocation_5 (Variables|Default|GetPrevLocation))
  (bind _prevlocation_6 (Variables|Default|GetPrevLocation))
  (bind _prevlocation_7 (Variables|Default|GetPrevLocation))
  (bind _prevlocation_8 (Variables|Default|GetPrevLocation))
  (bind _returnvalue (+ _roomsize_max 1))
  (bind _returnvalue_2 (select _merging _returnvalue _roomsize_max))
  (bind (_location _isfloortile) (Utilities|TestRelativeTileLocation _prevlocation_6 _returnvalue_2))
  (bind (_location_2 _isfloortile_2) (Utilities|TestRelativeTileLocation _prevlocation_7 0 _returnvalue_2))
  (bind (_location_3 _isfloortile_3) (Utilities|TestRelativeTileLocation _prevlocation_8 _returnvalue_2 _returnvalue_2))
  (bind _returnvalue_3 (* _returnvalue_2 -1))
  (bind (_location_4 _isfloortile_4) (Utilities|TestRelativeTileLocation _prevlocation_2 _returnvalue_3 _returnvalue_3))
  (bind (_location_5 _isfloortile_5) (Utilities|TestRelativeTileLocation _prevlocation_3 _returnvalue_3))
  (bind (_location_6 _isfloortile_6) (Utilities|TestRelativeTileLocation _prevlocation_4 _returnvalue_2 _returnvalue_3))
  (bind (_location_7 _isfloortile_7) (Utilities|TestRelativeTileLocation _prevlocation_5 0 _returnvalue_3))
  (bind (_location_8 _isfloortile_8) (Utilities|TestRelativeTileLocation _prevlocation _returnvalue_3 _returnvalue_2))
  (LocalVariables|SetDirections (Utilities|Array|MakeArray 0 1 2 3 4 5 6 7))
  (while (LocalVariables|GetSearching)
    ;[1 1 1] Make sure options available
    (if (>= (Utilities|Array|LastIndex (LocalVariables|GetDirections)) 0)
      (LocalVariables|SetTestIndex (Class|KismetMathLibrary|RandomIntegerfromStream (Variables|EditorTools|GetStream) (Utilities|Array|LastIndex (LocalVariables|GetDirections))))
      (if (Utilities|Select :Index (LocalVariables|GetTestIndex) :Option%200 _isfloortile :Option%201 _isfloortile_3 :Option%202 _isfloortile_2 :Option%203 _isfloortile_8 :Option%204 _isfloortile_5 :Option%205 _isfloortile_4 :Option%206 _isfloortile_7 :Option%207 _isfloortile_6)
        (Utilities|Array|RemoveIndex (LocalVariables|GetDirections) (LocalVariables|GetTestIndex))
        (LocalVariables|SetSearching true)
        (else
          (LocalVariables|SetSearching false)
          (LocalVariables|SetValid true)
          (LocalVariables|SetNewLocation (Utilities|Select :Index (LocalVariables|GetTestIndex) :Option%200 _location :Option%201 _location_3 :Option%202 _location_2 :Option%203 _location_8 :Option%204 _location_5 :Option%205 _location_4 :Option%206 _location_7 :Option%207 _location_6))))
      (else
        ;[1 1 1] Fail out and flag invalid
        (LocalVariables|SetSearching false)
        (LocalVariables|SetValid false))))
  (return (LocalVariables|GetValid) (LocalVariables|GetNewLocation)))