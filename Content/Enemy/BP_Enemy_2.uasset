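; BP_Enemy_2 is an enemy that chases the player and plays an attack animation on reaching them.
; When PawnSensing sees any pawn, it sets IsSeeingPlayer, which is never cleared here, and runs AIMoveTo toward player 0.
; On a successful move, the CanAttackPlayer flag gates the attack montage and re-enables after a delay equal to the montage's returned length.
; The graph applies no damage itself.
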(event OnSeePawn(PawnSensing)
  (params (Pawn :type Pawn%20Object%20Reference))
  (Variables|Default|SetisSeeingPlayer true)
  (CallFunction|FollowPlayer))

(event Custom|FollowPlayer
  (if (Variables|Default|GetisSeeingPlayer)
    (AI|AIMoveTo self "0, 0, 0" (Game|GetPlayerCharacter 0) 18.0 false
      (:OnSuccess
        (if (Variables|Default|GetcanAttackPlayer)
          (Variables|Default|SetcanAttackPlayer false)
          (bind _returnvalue (Animation|PlayAnimMontage "/Game/Enemy/Animation_Montages/Attack_Anim_Enemy_2.Attack_Anim_Enemy_2" 1.0 "None"))
          (Utilities|FlowControl|Delay _returnvalue)
          (Variables|Default|SetcanAttackPlayer true))))))

(event EventBeginPlay)

(event Collision|EventActorBeginOverlap
  (params (OtherActor :type Actor%20Object%20Reference)))

(event EventTick
  (params (DeltaSeconds :type Float%20%28single-precision%29)))

(fn ConstructionScript)